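; BP_Ghost is a ghost pawn that wanders the level and is destroyed when hit by a projectile.
; A self-repeating MoveGhost event uses AIMoveTo toward random reachable points around its current location, pausing after success and retrying quickly on failure.
; A hit from an actor tagged Projectile spawns an attached leaf-burst Niagara effect, hides the mesh and disables capsule collision, then destroys the ghost after a delay.
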(event `self.ReceiveBeginPlay`
  (`KismetSystemLibrary.Delay` 1.0)
  (`self.Move Ghost`))

(event `Move Ghost`
  (`|AIMoveTo` self (`NavigationSystemV1.K2_GetRandomReachablePointInRadius` (`self.K2_GetActorLocation`) 1000.0 null null) null
    (:`OnSuccess`
      (`KismetSystemLibrary.Delay` 4.0)
      (`self.Move Ghost`))
    (:`OnFail`
      (`KismetSystemLibrary.Delay` 0.2)
      (`self.Move Ghost`))))

(event `self.ReceiveHit`
  (params (MyComp :type "PrimitiveComponent Object Reference") (Other :type "Actor Object Reference") (OtherComp :type "PrimitiveComponent Object Reference") (bSelfMoved :type Boolean) (HitLocation :type "Vector Structure") (HitNormal :type "Vector Structure") (NormalImpulse :type "Vector Structure") (Hit :type "HitResult Structure (by ref)"))
  (if (`self.ActorHasTag` Other "Projectile")
    (`NiagaraFunctionLibrary.SpawnSystemAttached` "/Game/Niagara/NS_BurstLeaf.NS_BurstLeaf" MyComp "None" (0.0 0.0 0.0) (struct) "KeepRelativeOffset")
    (`SceneComponent.SetVisibility` (`self.Mesh`) false false)
    (`PrimitiveComponent.SetCollisionEnabled` (`self.Capsule`) "NoCollision")
    (`KismetSystemLibrary.Delay` 4.0)
    (`self.K2_DestroyActor`)))

(fn `UserConstructionScript`)